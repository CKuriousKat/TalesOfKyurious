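; AshbringerBlueBP is a blue Ashbringer weapon actor that the player can pick up and carry.
; Its PickUp event detaches any weapon the ThirdPersonCharacter already has equipped and moves it to this weapon's location and rotation, swapping the two.
; It then registers itself as EquippedWeapon and snaps onto the character mesh's weapon_back socket.
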(event EventPickUp
  (bind _returnvalue (Game|GetPlayerCharacter 0))
  (bind _defaultsceneroot (Variables|Default|GetDefaultSceneRoot))
  (bind _asthird_person_character (Utilities|Casting|CastToThirdPersonCharacter _returnvalue))
  (Utilities|IsValid (Variables|/Game/ThirdPersonBP/Blueprints/ThirdPersonCharacter.ThirdPersonCharacter_C|GetEquippedWeapon _asthird_person_character)
    (:Is%20Valid
      (Transformation|DetachFromActor (Variables|/Game/ThirdPersonBP/Blueprints/ThirdPersonCharacter.ThirdPersonCharacter_C|GetEquippedWeapon _asthird_person_character) "KeepRelative" "KeepRelative" "KeepRelative")
      (Transformation|SetActorLocationAndRotation (Variables|/Game/ThirdPersonBP/Blueprints/ThirdPersonCharacter.ThirdPersonCharacter_C|GetEquippedWeapon _asthird_person_character) (Transformation|GetWorldLocation _defaultsceneroot) (Transformation|GetWorldRotation _defaultsceneroot)))
    (:Is%20Not%20Valid
      _))
  (Variables|/Game/ThirdPersonBP/Blueprints/ThirdPersonCharacter.ThirdPersonCharacter_C|SetEquippedWeapon _asthird_person_character self)
  (Transformation|AttachComponentToComponent (Variables|/Script/Engine.Character|GetMesh _asthird_person_character) "weapon_back" "SnapToTarget" "SnapToTarget" "KeepRelative" true))

(fn ConstructionScript)