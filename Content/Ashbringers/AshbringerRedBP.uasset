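; Red Ashbringer weapon Blueprint that the player can pick up, swapping it with any weapon already equipped.
; Its PickUp event casts the player character to NPC, then detaches a valid EquippedWeapon and moves it to this weapon's current location and rotation.
; It then records itself as EquippedWeapon and attaches to the weapon_back socket on the character's mesh.
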(event EventPickUp
  (bind _returnvalue (Game|GetPlayerCharacter 0))
  (bind _defaultsceneroot (Variables|Default|GetDefaultSceneRoot))
  (bind _asnpc (Utilities|Casting|CastToNPC _returnvalue))
  (Utilities|IsValid (Variables|/Game/NPC/NPC.NPC_C|GetEquippedWeapon _asnpc)
    (:Is%20Valid
      (Transformation|DetachFromActor (Variables|/Game/NPC/NPC.NPC_C|GetEquippedWeapon _asnpc) "KeepRelative" "KeepRelative" "KeepRelative")
      (Transformation|SetActorLocationAndRotation (Variables|/Game/NPC/NPC.NPC_C|GetEquippedWeapon _asnpc) (Transformation|GetWorldLocation _defaultsceneroot) (Transformation|GetWorldRotation _defaultsceneroot)))
    (:Is%20Not%20Valid
      _))
  (Variables|/Game/NPC/NPC.NPC_C|SetEquippedWeapon _asnpc self)
  (Transformation|AttachComponentToComponent (Variables|/Script/Engine.Character|GetMesh _asnpc) "weapon_back" "SnapToTarget" "SnapToTarget" "KeepRelative" true))

(fn ConstructionScript)