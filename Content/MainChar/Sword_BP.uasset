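; Sword weapon Blueprint that deals fixed melee damage to actors entering its HitRange while an attack is active.
; AttackInitiated and AttackNotInitiated events toggle the attack flag, and a DoOnce with a delayed reset throttles hits.
; The overlap path applies no tag filter.
; Pickup and Hit events are empty; their weapon-swap socket attachment and random damage against Enemy-tagged actors sit in unconnected, never-run nodes.
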(event OnComponentBeginOverlap(HitRange)
  (params (OverlappedComponent :type Primitive%20Component%20Object%20Reference) (OtherActor :type Actor%20Object%20Reference) (OtherComp :type Primitive%20Component%20Object%20Reference) (OtherBodyIndex :type Integer) (bFromSweep :type Boolean) (SweepResult :type Hit%20Result%20Structure%20%28by%20ref%29))
  (if (Variables|Default|GetAttackInitiated_0)
    (Utilities|FlowControl|DoOnce false :!label _label
      (:Completed
        (Game|Damage|ApplyDamage OtherActor 5e+01 0 self)
        (Utilities|FlowControl|Delay 0.5)
        (goto _label Reset)))))

(event EventPickup
  ;[1 1 1] Pickup/Swan Weapon
)

(event Collision|EventHit
  (params (MyComp :type Primitive%20Component%20Object%20Reference) (Other :type Actor%20Object%20Reference) (OtherComp :type Primitive%20Component%20Object%20Reference) (bSelfMoved :type Boolean) (HitLocation :type Vector :default "0, 0, 0") (HitNormal :type Vector :default "0, 0, 0") (NormalImpulse :type Vector :default "0, 0, 0") (Hit :type Hit%20Result%20Structure%20%28by%20ref%29))
  ;[1 1 1] NOT WORKING
)

(event EventAttackInitiated
  (Variables|Default|SetAttackInitiated_0 true))

(event EventAttackNotInitiated
  (Variables|Default|SetAttackInitiated_0 false))

(fn ConstructionScript)